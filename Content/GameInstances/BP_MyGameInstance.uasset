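; Game instance Blueprint that shows the main menu and holding screen widgets.
; Each event creates its widget for the first player controller only when no valid cached reference exists, then adds it to the viewport.
; ShowMainMenu turns the mouse cursor on and ShowHolding turns it off.
; Neither event removes the other widget or changes the input mode.
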(event Custom|ShowMainMenu
  (bind _returnvalue (Game|GetPlayerController 0))
  (Utilities|IsValid (Variables|Default|GetMenu)
    (:Is%20Valid
      _)
    (:Is%20Not%20Valid
      (bind _returnvalue_2 (UserInterface|CreateWidget "/Game/UI/WBP_Menu.WBP_Menu_C" _returnvalue))
      (Variables|Default|SetMenu _returnvalue_2)))
  (UserInterface|Viewport|AddtoViewport (Variables|Default|GetMenu) 0)
  (Variables|/Script/Engine.PlayerController|SetbShowMouseCursor _returnvalue true))

(event Custom|ShowHolding
  (bind _returnvalue (Game|GetPlayerController 0))
  (Utilities|IsValid (Variables|Default|GetHolding)
    (:Is%20Valid
      _)
    (:Is%20Not%20Valid
      (bind _returnvalue_2 (UserInterface|CreateWidget "/Game/UI/WBP_Holding.WBP_Holding_C" _returnvalue))
      (Variables|Default|SetHolding _returnvalue_2)))
  (UserInterface|Viewport|AddtoViewport (Variables|Default|GetHolding) 0)
  (Variables|/Script/Engine.PlayerController|SetbShowMouseCursor _returnvalue false))